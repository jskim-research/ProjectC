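; Behavior tree service for AI cluster behavior, so far only caching role-based character lists and printing debug output.
; On activation it reads Tank, Healer and Dealer array objects from blackboard keys, casts them to BlackboardCharacterArrayObject and stores them, stopping at the first failed cast.
; It then prints each element of the Dealer array and a completion message, while Tick is empty.
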(event `self.ReceiveActivation`
  (params (OwnerActor :type "Actor Object Reference"))
  (bind _asblackboard_character_array_object (cast `BlackboardCharacterArrayObject` (`BTFunctionLibrary.GetBlackboardValueAsObject` (`self.TankArrayKey`))))
  (set `self.TankArray` _asblackboard_character_array_object)
  (bind _asblackboard_character_array_object_2 (cast `BlackboardCharacterArrayObject` (`BTFunctionLibrary.GetBlackboardValueAsObject` (`self.HealerArrayKey`))))
  (set `self.HealerArray` _asblackboard_character_array_object_2)
  (bind _asblackboard_character_array_object_3 (cast `BlackboardCharacterArrayObject` (`BTFunctionLibrary.GetBlackboardValueAsObject` (`self.DealerArrayKey`))))
  (bind _output_get (set `self.DealerArray` _asblackboard_character_array_object_3))
  (for (_ _array_index) (`BlackboardCharacterArrayObject.CharacterArray` _output_get)
    (`KismetSystemLibrary.PrintString` (`KismetStringLibrary.Conv_IntToString` _array_index)))
  (`KismetSystemLibrary.PrintString` "Complete"))

(event `self.ReceiveTick`
  (params (OwnerActor :type "Actor Object Reference") (DeltaSeconds :type "Float (single-precision)")))