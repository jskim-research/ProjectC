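; Base projectile actor that destroys itself after traveling MaxRange from its spawn point or on any Box overlap.
; BeginPlay stores the start location, and Tick compares the straight-line distance from it against MaxRange.
; Overlap only prints a debug string before destruction, as the ApplyDamage call is disconnected.
; EnableCollision switches the Box to query and physics collision, with no caller in this file.
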(event `self.ReceiveBeginPlay`
  (set `self.StartLocation` (`self.K2_GetActorLocation`)))

(event `self.ReceiveTick`
  (params (DeltaSeconds :type "Float (single-precision)"))
  (if (>= (`KismetMathLibrary.Vector_Distance` (`self.K2_GetActorLocation`) (`self.StartLocation`)) (`self.MaxRange`))
    (`self.K2_DestroyActor`)))

(event `self.Box.OnComponentBeginOverlap`
  (params (OverlappedComponent :type "PrimitiveComponent Object Reference") (OtherActor :type "Actor Object Reference") (OtherComp :type "PrimitiveComponent Object Reference") (OtherBodyIndex :type Integer) (bFromSweep :type Boolean) (SweepResult :type "HitResult Structure (by ref)"))
  ;[1 1 1] Interaction 과의 overlap 겹침 방지를 위해 PlayerMesh 와의 충돌만 체크
  (`KismetSystemLibrary.PrintString` "Overlap!")
  (`self.K2_DestroyActor`))

(fn `EnableCollision`
  (`PrimitiveComponent.SetCollisionEnabled` (`self.Box`) "QueryAndPhysics"))

(fn `UserConstructionScript`)